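; BP_DoorRight is a lobby door that swings open when a journalist carrying the matching key enters its overlap volume.
; The overlap checks the journalist's OwnedKeys against RequiredKeyType.
; On a match, it copies those keys into GameInstanceKeys and plays a timeline that drives the door's relative yaw.
; The door has no closing logic.
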(event `self.Overlap.OnComponentBeginOverlap`
  (params (OverlappedComponent :type "PrimitiveComponent Object Reference") (OtherActor :type "Actor Object Reference") (OtherComp :type "PrimitiveComponent Object Reference") (OtherBodyIndex :type Integer) (bFromSweep :type Boolean) (SweepResult :type "HitResult Structure (by ref)"))
  (bind _asbp_journalist (cast `/Game/_Game/Lobby_Resources/Blueprints/BP_Journalist` OtherActor))
  (bind _ownedkeys (`/Game/_Game/Lobby_Resources/Blueprints/BP_Journalist.OwnedKeys` _asbp_journalist))
  (for _array_element _ownedkeys
    (if (`|EnumEquality` _array_element (`self.RequiredKeyType`))
      (bind _asgame_instance_keys (cast `/Game/_Game/Lobby_Resources/GameInstanceKeys` (`GameplayStatics.GetGameInstance`)))
      (set `/Game/_Game/Lobby_Resources/GameInstanceKeys.PlayerKeys` _ownedkeys _asgame_instance_keys)
      (bind (_direction _newtrack_0) (`Timeline|Timeline_0`)
        (:`Update`
          (`SceneComponent.K2_SetRelativeRotation` (`self.Door`) (`KismetMathLibrary.MakeRotator` 0.0 0.0 _newtrack_0) false false))))))

(fn `UserConstructionScript`)