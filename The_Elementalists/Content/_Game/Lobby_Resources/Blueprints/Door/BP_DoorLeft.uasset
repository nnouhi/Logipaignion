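; BP_DoorLeft is a key-locked lobby door that swings open when a BP_Journalist carrying the required key type overlaps it.
; A match copies the player's keys to GameInstanceKeys and, if unrotated, plays a sound and timeline-driven yaw rotation.
; A non-match on the last key shows a no-access widget, then removes all widgets after a delay.
; Tick polls the game instance's Finale flag to drive a second rotation timeline.
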(event `self.Overlap.OnComponentBeginOverlap`
  (params (OverlappedComponent :type "PrimitiveComponent Object Reference") (OtherActor :type "Actor Object Reference") (OtherComp :type "PrimitiveComponent Object Reference") (OtherBodyIndex :type Integer) (bFromSweep :type Boolean) (SweepResult :type "HitResult Structure (by ref)"))
  (bind _asbp_journalist (cast `/Game/_Game/Lobby_Resources/Blueprints/Player/BP_Journalist` OtherActor))
  (bind _ownedkeys (`/Game/_Game/Lobby_Resources/Blueprints/Player/BP_Journalist.OwnedKeys` _asbp_journalist))
  (for (_array_element _array_index) _ownedkeys
    (if (`|EnumEquality` _array_element (`self.RequiredKeyType`))
      (bind _asgame_instance_keys (cast `/Game/_Game/Lobby_Resources/GameInstanceKeys` (`GameplayStatics.GetGameInstance`)))
      (set `/Game/_Game/Lobby_Resources/GameInstanceKeys.PlayerKeys` _ownedkeys _asgame_instance_keys)
      (if (`self.Not Rotated`)
        (`GameplayStatics.PlaySound2D` "/Game/_Game/Door_Open_WAV.Door_Open_WAV" 0.5 1.0 0.0 null null)
        (bind (_direction _newtrack_0) (`Timeline|Timeline_0`)
          (:`Update`
            (`SceneComponent.K2_SetRelativeRotation` (`self.Door`) (`KismetMathLibrary.MakeRotator` 0.0 0.0 _newtrack_0) false false)
            (set `self.Not Rotated` false))))
      (elif (and (== _array_index (`KismetArrayLibrary.Array_LastIndex` _ownedkeys)) (`self.Not Rotated`))
        (bind _returnvalue (`|CreateWidget` "/Game/_Game/Lobby_Resources/NoAccessWidget.NoAccessWidget_C"))
        (`UserWidget.AddToViewport` _returnvalue 0)
        (`KismetSystemLibrary.Delay` 3.0)
        (`WidgetLayoutLibrary.RemoveAllWidgets`)))))

(event `self.ReceiveTick`
  (params (DeltaSeconds :type "Float (single-precision)"))
  (bind _asgame_instance_keys (cast `/Game/_Game/Lobby_Resources/GameInstanceKeys` (`GameplayStatics.GetGameInstance`)))
  (if (`/Game/_Game/Lobby_Resources/GameInstanceKeys.Finale` _asgame_instance_keys)
    (bind (_direction _newtrack_0) (`Timeline|Timeline_1`)
      (:`Update`
        (`SceneComponent.K2_SetRelativeRotation` (`self.Door`) (`KismetMathLibrary.MakeRotator` 0.0 0.0 _newtrack_0) false false)))))

(fn `UserConstructionScript`)