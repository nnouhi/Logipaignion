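; BP_Journalist is the journalist actor in the lobby resources, handling player interaction and owned keys.
; On BeginPlay it loads OwnedKeys from the GameInstanceKeys game instance and appends one fixed key.
; Its InteractionSphere overlaps track InteractionInterface implementers, checking the overlapping actor first and otherwise its components.
; Pressing Interact calls OnInteraction on the first tracked entry, passing itself, with no distance sorting.
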(event `self.ReceiveBeginPlay`
  (bind _asgame_instance_keys (cast `/Game/_Game/Lobby_Resources/GameInstanceKeys` (`GameplayStatics.GetGameInstance`)))
  (set `self.OwnedKeys` (`/Game/_Game/Lobby_Resources/GameInstanceKeys.PlayerKeys` _asgame_instance_keys))
  (`KismetArrayLibrary.Array_Add` (`self.OwnedKeys`) "NewEnumerator5"))

(event `self.InteractionSphere.OnComponentBeginOverlap`
  (params (OverlappedComponent :type "PrimitiveComponent Object Reference") (OtherActor :type "Actor Object Reference") (OtherComp :type "PrimitiveComponent Object Reference") (OtherBodyIndex :type Integer) (bFromSweep :type Boolean) (SweepResult :type "HitResult Structure (by ref)"))
  (bind _asinteraction_interface (cast `/Game/_Game/Lobby_Resources/Interact/InteractionInterface` OtherActor)
    (:`then`
      (`KismetArrayLibrary.Array_AddUnique` (`self.InteractablesInRange`) _asinteraction_interface))
    (:`CastFailed`
      (for _array_element (`self.GetComponentsByInterface` OtherActor "/Game/_Game/Lobby_Resources/Interact/InteractionInterface.InteractionInterface_C")
        (`KismetArrayLibrary.Array_AddUnique` (`self.InteractablesInRange`) (cast `/Game/_Game/Lobby_Resources/Interact/InteractionInterface` _array_element :!pure true))))))

(event `self.InteractionSphere.OnComponentEndOverlap`
  (params (OverlappedComponent :type "PrimitiveComponent Object Reference") (OtherActor :type "Actor Object Reference") (OtherComp :type "PrimitiveComponent Object Reference") (OtherBodyIndex :type Integer))
  (bind _asinteraction_interface (cast `/Game/_Game/Lobby_Resources/Interact/InteractionInterface` OtherActor)
    (:`then`
      (`KismetArrayLibrary.Array_RemoveItem` (`self.InteractablesInRange`) _asinteraction_interface))
    (:`CastFailed`
      (for _array_element (`self.GetComponentsByInterface` OtherActor "/Game/_Game/Lobby_Resources/Interact/InteractionInterface.InteractionInterface_C")
        (`KismetArrayLibrary.Array_RemoveItem` (`self.InteractablesInRange`) (cast `/Game/_Game/Lobby_Resources/Interact/InteractionInterface` _array_element :!pure true))))))

(event `InputAction|Interact`
  (params (Key :type "Key Structure"))
  (:`Pressed`
    (if (> (`KismetArrayLibrary.Array_Length` (`self.InteractablesInRange`)) 0)
      (`/Game/_Game/Lobby_Resources/Interact/InteractionInterface.OnInteraction` (`|GetArrayItem` (`self.InteractablesInRange`)) self))))

(fn `UserConstructionScript`)