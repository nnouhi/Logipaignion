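; BP_Endpoint is an overlap trigger for flashback levels that marks that chapter's questions as available.
; On any actor overlap, it compares the current level name against the flashback levels for chapters one to three in a chain of branches.
; The matching branch casts the game instance to GameInstanceKeys and sets that chapter's QuestionAvailability variable.
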(event `self.ReceiveActorBeginOverlap`
  (params (OtherActor :type "Actor Object Reference"))
  (bind _returnvalue (`GameplayStatics.GetCurrentLevelName` true))
  (if (== _returnvalue "Chapter_1_Flashback")
    (bind _asgame_instance_keys (cast `/Game/_Game/Lobby_Resources/GameInstanceKeys` (`GameplayStatics.GetGameInstance`)))
    (set `/Game/_Game/Lobby_Resources/GameInstanceKeys.QuestionAvailabilityChapter1` 1 _asgame_instance_keys)
    (else
      (bind _returnvalue_2 (`GameplayStatics.GetCurrentLevelName` true))
      (if (== _returnvalue_2 "Chapter_2_Flashback")
        (bind _asgame_instance_keys_2 (cast `/Game/_Game/Lobby_Resources/GameInstanceKeys` (`GameplayStatics.GetGameInstance`)))
        (set `/Game/_Game/Lobby_Resources/GameInstanceKeys.QuestionAvailabilityChapter2` 1 _asgame_instance_keys_2)
        (else
          (bind _returnvalue_3 (`GameplayStatics.GetCurrentLevelName` true))
          (if (== _returnvalue_3 "Chapter_3_Flashback")
            (bind _asgame_instance_keys_3 (cast `/Game/_Game/Lobby_Resources/GameInstanceKeys` (`GameplayStatics.GetGameInstance`)))
            (set `/Game/_Game/Lobby_Resources/GameInstanceKeys.QuestionAvailabilityChapter3` 1 _asgame_instance_keys_3)))))))

(fn `UserConstructionScript`)