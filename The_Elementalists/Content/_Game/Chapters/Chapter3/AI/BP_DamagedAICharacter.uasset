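; BP_DamagedAICharacter is a Chapter 3 AI character with a health component and an overhead-style health bar widget.
; On BeginPlay it registers itself as the Owner of its WBP_AIHealthBar.
; The MakeVisible overlap volume shows the bar while BP_Chapter3Character is inside and hides it on exit.
; Tick polls health and, at zero or below, calls ActorDied on BaseGameMode, with no guard against repeat calls.
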(event `self.ReceiveBeginPlay`
  (bind _aswbp_aihealth_bar (cast `/Game/_Game/Chapters/Chapter3/AI/WBP_AIHealthBar` (`WidgetComponent.GetUserWidgetObject` (`self.Healthbar`))))
  (set `/Game/_Game/Chapters/Chapter3/AI/WBP_AIHealthBar.Owner` self _aswbp_aihealth_bar))

(event `self.ReceiveTick`
  (params (DeltaSeconds :type "Float (single-precision)"))
  (if (<= (`HealthComponent.GetHealthPercentage` (`self.Health`)) 0.0)
    (bind _asbase_game_mode (cast `BaseGameMode` (`GameplayStatics.GetGameMode`)))
    (`BaseGameMode.ActorDied` _asbase_game_mode self)))

(event `self.MakeVisible.OnComponentBeginOverlap`
  (params (OverlappedComponent :type "PrimitiveComponent Object Reference") (OtherActor :type "Actor Object Reference") (OtherComp :type "PrimitiveComponent Object Reference") (OtherBodyIndex :type Integer) (bFromSweep :type Boolean) (SweepResult :type "HitResult Structure (by ref)"))
  (cast `/Game/_Game/Chapters/Chapter3/Blueprints/BP_Chapter3Character` OtherActor)
  (`SceneComponent.SetVisibility` (`self.Healthbar`) true false))

(event `self.MakeVisible.OnComponentEndOverlap`
  (params (OverlappedComponent :type "PrimitiveComponent Object Reference") (OtherActor :type "Actor Object Reference") (OtherComp :type "PrimitiveComponent Object Reference") (OtherBodyIndex :type Integer))
  (cast `/Game/_Game/Chapters/Chapter3/Blueprints/BP_Chapter3Character` OtherActor)
  (`SceneComponent.SetVisibility` (`self.Healthbar`) false false))

(fn `UserConstructionScript`)