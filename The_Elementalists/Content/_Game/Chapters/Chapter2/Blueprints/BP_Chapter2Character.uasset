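; Chapter 2 player character with a minimap and an F-key pulse that highlights specific objects.
; On BeginPlay, the minimap scene capture hides the character's mesh.
; F restarts a timeline that drives the PC_Radius parameter collection and scales a WorldDynamic sphere trace, activating any BP_Test it hits.
; Each trace returns one hit and ends at the mesh location with X and Y zeroed, not at the character.
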(event `self.ReceiveBeginPlay`
  ;[1 1 1] Make scene capture comp hide the player
  (`SceneCaptureComponent.HideComponent` (`self.Minimap`) (`self.Mesh`)))

(event `Key|F`
  (params (Key :type "Key Structure"))
  (bind _returnvalue (`SceneComponent.K2_GetComponentLocation` (`self.Mesh`)))
  ;[1 1 1] Highlight specific objects when F key is pressed
  (:`Pressed`
    (bind (_direction _newtrack_0) (`Timeline|Timeline_0` :!via `PlayFromStart`)
      (:`Update`
        (`KismetMaterialLibrary.SetScalarParameterValue` "/Game/_Game/Chapters/Chapter1/ScanEffect/PC_Radius.PC_Radius" "Radius" _newtrack_0)
        (bind _outhit (`KismetSystemLibrary.SphereTraceSingleForObjects` _returnvalue (* _returnvalue (0.0 0.0 1.0)) (* _newtrack_0 5000.0) (`|MakeArray` "ObjectTypeQuery2" :!type "EObjectTypeQuery Enum")))
        (bind _asbp_test (cast `/Game/_Game/Chapters/Chapter1/ScanEffect/BP_Test` (`.HitActor` (`GameplayStatics.BreakHitResult` _outhit))))
        (`/Game/_Game/Chapters/Chapter1/ScanEffect/BP_Test.Activate` _asbp_test)))))

(fn `UserConstructionScript`)