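; Chapter 1 character Blueprint that adds a minimap and an F-key highlight pulse for specific objects.
; On BeginPlay, the Minimap scene capture hides the character's mesh.
; Pressing F plays a timeline that drives the Radius scalar in the PC_Radius parameter collection.
; The timeline's update also sets StencilValue on GameInstanceKeys to 2, then back to 0 after a three-second delay.
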(event `self.ReceiveBeginPlay`
  ;[1 1 1] Make scene capture comp hide the player
  (`SceneCaptureComponent.HideComponent` (`self.Minimap`) (`self.Mesh`)))

(event `Key|F`
  (params (Key :type "Key Structure"))
  ;[1 1 1] Highlight specific objects when F key is pressed
  (:`Pressed`
    (bind (_direction _newtrack_0) (`Timeline|Timeline_0` :!via `PlayFromStart`)
      (:`Update`
        (`KismetMaterialLibrary.SetScalarParameterValue` "/Game/_Game/Chapters/Chapter1/ScanEffect/PC_Radius.PC_Radius" "Radius" _newtrack_0)
        (bind _asgame_instance_keys (cast `/Game/_Game/Lobby_Resources/GameInstanceKeys` (`GameplayStatics.GetGameInstance`)))
        (set `/Game/_Game/Lobby_Resources/GameInstanceKeys.StencilValue` 2 _asgame_instance_keys)
        (`KismetSystemLibrary.Delay` 3.0)
        (set `/Game/_Game/Lobby_Resources/GameInstanceKeys.StencilValue` 0 _asgame_instance_keys)))))

(fn `UserConstructionScript`)