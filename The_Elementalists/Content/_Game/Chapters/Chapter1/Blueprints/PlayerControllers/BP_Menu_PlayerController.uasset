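; Player controller for a Chapter 1 menu that slowly drifts and turns the first player's pawn, with no input handling.
; Tick moves the pawn along world +Y at a constant rate scaled by delta time, without sweeping.
; It also nudges the pawn's forward vector toward world -Y each frame and rebuilds its rotation through MakeRotationFromAxes, passing zero Right and Up vectors.
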(event `self.ReceiveTick`
  (params (DeltaSeconds :type "Float (single-precision)"))
  (bind _returnvalue (`GameplayStatics.GetPlayerPawn` 0))
  (bind _returnvalue_2 (`GameplayStatics.GetPlayerPawn` 0))
  (`self.K2_SetActorLocation` _returnvalue (+ (* (0.0 10.0 0.0) DeltaSeconds) (`self.K2_GetActorLocation` _returnvalue)) false false)
  (`self.K2_SetActorRotation` _returnvalue_2 (`KismetMathLibrary.MakeRotationFromAxes` (+ (* (0.0 -0.1 0.0) DeltaSeconds) (`KismetMathLibrary.GetForwardVector` (`self.K2_GetActorRotation` _returnvalue_2)))) false))

(fn `UserConstructionScript`)